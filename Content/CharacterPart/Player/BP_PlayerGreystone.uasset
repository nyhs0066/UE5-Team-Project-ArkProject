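; Player character Blueprint for Greystone with cursor-aimed attacks.
; Each tick, a cursor component follows the visibility trace under the mouse at a fixed height, aligned to the impact normal.
; Fire stops movement and, unless skill or aim is active, flags an attack on the anim Blueprint and turns the character's yaw toward the cursor if not already attacking.
; The Skill_E input has no effect.
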(event `self.ReceiveBeginPlay`
  (`parent.ReceiveBeginPlay`)
  (cast `/Game/CharacterPart/Player/Anim/BP_GreystoneAnim` (`SkeletalMeshComponent.GetAnimInstance` (`self.Mesh`))))

(event `self.ReceiveTick`
  (params (DeltaSeconds :type "Float (single-precision)"))
  (bind (_bblockinghit _binitialoverlap _time _distance _location _impactpoint _normal _impactnormal) (`GameplayStatics.BreakHitResult` (`PlayerController.GetHitResultUnderCursorByChannel` (`GameplayStatics.GetPlayerController` 0) "TraceTypeQuery1" true)))
  (`parent.ReceiveTick` DeltaSeconds)
  (`SceneComponent.K2_SetWorldLocationAndRotation` (`self.Cursor`) (`KismetMathLibrary.MakeVector` (.x _location) (.y _location) 270.0) (`KismetMathLibrary.Conv_VectorToRotator` _impactnormal) false false))

(event `InputAction|Fire`
  (params (Key :type "Key Structure"))
  (:`Pressed`
    (`NavMovementComponent.StopActiveMovement` (`self.CharacterMovement`))
    (if (`self.Skill_On`)
      _
      (elif (not (`self.AimOn`))
        (`self.Attack`)
        (if (`self.CharacterSpin`)
          (`self.PlayerSpin`))))))

(event `Attack`
  (bind _animbp_1 (`self.AnimBP_1`))
  (set `self.CanMove` false)
  (if (`/Game/CharacterPart/Player/Anim/BP_GreystoneAnim.IsAttack` _animbp_1)
    (set `self.CharacterSpin` false)
    (else
      (set `self.CharacterSpin` true)
      (set `/Game/CharacterPart/Player/Anim/BP_GreystoneAnim.IsAttack` true _animbp_1))))

(event `InputAction|Skill_E`
  (params (Key :type "Key Structure"))
  (:`Pressed`
    (if true
      _)))

(fn `PlayerSpin`
  (bind (_returnvalue_roll _returnvalue_pitch _returnvalue_yaw) (`KismetMathLibrary.BreakRotator` (`KismetMathLibrary.FindLookAtRotation` (`SceneComponent.K2_GetComponentLocation` (`self.Mesh`)) (`SceneComponent.K2_GetComponentLocation` (`self.Cursor`)))))
  (`self.K2_SetActorRotation` self (`KismetMathLibrary.MakeRotator` 0.0 0.0 _returnvalue_yaw) false))

(fn `UserConstructionScript`
  (`parent.UserConstructionScript`))