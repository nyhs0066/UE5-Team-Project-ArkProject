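; Damage-area actor for the Revenent player's W skill that hits bosses repeatedly over a short lifetime.
; BeginPlay runs a delayed loop that toggles the box collision off and straight back on to retrigger overlaps, then destroys the actor after a fixed count.
; Overlaps with a BP_Boss other than the instigator apply damage and play an impact sound.
; SetDamage stores the damage type and a multiplied damage value.
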(event `self.ReceiveBeginPlay`
  (bind _count (`self.Count`))
  (`PrimitiveComponent.SetCollisionEnabled` (`self.Box`) "QueryAndPhysics" :!label _label)
  (`KismetSystemLibrary.Delay` 0.1)
  (set `self.Count` (+ _count 1))
  (if (> _count 6)
    (`self.K2_DestroyActor`)
    (else
      (`PrimitiveComponent.SetCollisionEnabled` (`self.Box`) "NoCollision")
      (goto _label))))

(event `self.ReceiveTick`
  (params (DeltaSeconds :type "Float (single-precision)")))

(event `self.Box.OnComponentBeginOverlap`
  (params (OverlappedComponent :type "PrimitiveComponent Object Reference") (OtherActor :type "Actor Object Reference") (OtherComp :type "PrimitiveComponent Object Reference") (OtherBodyIndex :type Integer) (bFromSweep :type Boolean) (SweepResult :type "HitResult Structure (by ref)"))
  (if (!= OtherActor (`self.GetInstigator`))
    (bind _asbp_boss (cast `/Game/BossPart/BP_Boss` OtherActor))
    (`GameplayStatics.ApplyDamage` _asbp_boss (`self.Damage`) null null (`GameplayStatics.GetObjectClass` (`self.DamageType`)))
    (`GameplayStatics.PlaySoundAtLocation` "/Game/Resource/Sound/Character/Tychus_Attack_Impact_Multi_Stone02.Tychus_Attack_Impact_Multi_Stone02" (`self.K2_GetActorLocation`) (struct) 1.0 1.0 0.0 null null null null)))

(fn `SetDamage`
  (params (DamageType :type "DamageType Object Reference") (Damage :type "Float (double-precision)"))
  (set `self.DamageType` DamageType)
  (set `self.Damage` (* Damage 5.0)))

(fn `UserConstructionScript`)