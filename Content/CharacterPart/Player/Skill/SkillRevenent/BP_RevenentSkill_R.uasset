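; Revenant R skill actor that hits bosses with a short burst of repeated area impacts, then destroys itself.
; BeginPlay loops four timed pulses, each replaying particles and an impact sound and toggling sphere collision to retrigger overlaps.
; Overlaps apply damage only to non-instigator BP_Boss actors, re-randomizing the stored Damage each time so the variance accumulates.
; SetDamage supplies the damage type and triples the incoming damage.
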(event `self.ReceiveBeginPlay`
  (bind _count (`self.Count`))
  (`ActorComponent.Activate` (`self.ParticleSystem`) false :!label _label)
  (`GameplayStatics.PlaySoundAtLocation` "/Game/Resource/Sound/Character/Revenent/Tychus_Odin_Missile_Impact01.Tychus_Odin_Missile_Impact01" (`self.K2_GetActorLocation`) (struct) 1.0 1.0 0.0 null null null null)
  (`PrimitiveComponent.SetCollisionEnabled` (`self.Sphere`) "QueryAndPhysics")
  (`KismetSystemLibrary.Delay` 0.3)
  (set `self.Count` (+ _count 1))
  (`ActorComponent.Deactivate` (`self.ParticleSystem`))
  (if (> _count 3)
    (`self.K2_DestroyActor`)
    (else
      (`PrimitiveComponent.SetCollisionEnabled` (`self.Sphere`) "NoCollision")
      (goto _label))))

(event `self.Sphere.OnComponentBeginOverlap`
  (params (OverlappedComponent :type "PrimitiveComponent Object Reference") (OtherActor :type "Actor Object Reference") (OtherComp :type "PrimitiveComponent Object Reference") (OtherBodyIndex :type Integer) (bFromSweep :type Boolean) (SweepResult :type "HitResult Structure (by ref)"))
  (set `self.Damage` (`KismetMathLibrary.RandomFloatInRange` (- (`self.Damage`) 100000.0) (+ (`self.Damage`) 100000.0)))
  (if (!= OtherActor (`self.GetInstigator`))
    (bind _asbp_boss (cast `/Game/BossPart/BP_Boss` OtherActor))
    (`GameplayStatics.ApplyDamage` _asbp_boss (`self.Damage`) null null (`GameplayStatics.GetObjectClass` (`self.DamageType`)))))

(fn `SetDamage`
  (params (DamageType :type "DamageType Object Reference") (Damage :type "Float (double-precision)"))
  (set `self.DamageType` DamageType)
  (set `self.Damage` (* Damage 3.0)))

(fn `UserConstructionScript`)