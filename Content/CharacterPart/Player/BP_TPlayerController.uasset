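; Player controller for click-to-move and a cursor-aimed dodge on BP_BasePlayerChara.
; BeginPlay adds the Enhanced Input mapping; holding the click paths toward the cursor hit via SimpleMoveToLocation, while a short press also spawns a cursor effect.
; Dash checks cooldown and skill state, locks movement, calls Dodge, then slides the capsule toward the cursor, ending at a line-trace hit or full dash distance.
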(event `self.ReceiveTick`
  (params (DeltaSeconds :type "Float (single-precision)")))

(event `self.ReceiveBeginPlay`
  (bind _returnvalue (subsystem `EnhancedInputLocalPlayerSubsystem`))
  (`/Engine/EditorBlueprintResources/StandardMacros.IsValid` _returnvalue
    (:`Is Valid`
      (`EnhancedInputSubsystemInterface.AddMappingContext` _returnvalue "/Game/CharacterPart/Player/Input/IMC_MurielDefault.IMC_MurielDefault" 0 (struct))
      (bind _asbp_base_player_chara (cast `/Game/CharacterPart/Player/BP_BasePlayerChara` (`GameplayStatics.GetPlayerCharacter` 0)))
      (set `self.PlayerChara` _asbp_base_player_chara))))

(event `EnhancedInput|/Game/CharacterPart/Player/Input/IA_MoveClick`
  (params (ActionValue :type Boolean) (ElapsedSeconds :type "Float (double-precision)") (TriggeredSeconds :type "Float (double-precision)") (InputAction :type "InputAction Object Reference" :default "/Game/CharacterPart/Player/Input/IA_MoveClick.IA_MoveClick"))
  (bind (_location _hit) (`self.Get Location Under Cursor`))
  (bind _cacheddestination (`self.CachedDestination`))
  (:`Triggered`
    (bind _asbp_base_player_chara (cast `/Game/CharacterPart/Player/BP_BasePlayerChara` (`self.K2_GetPawn`)))
    (if (`/Game/CharacterPart/Player/BP_BasePlayerChara.CanMove` _asbp_base_player_chara)
      (if _hit
        (bind _output_get (set `self.CachedDestination` _location))
        (`self.MoveToLocation` _output_get))))
  (:`Canceled`
    (if (< ElapsedSeconds (`self.PressedThreshold`)) :!label _label
      (bind _asbp_base_player_chara_2 (cast `/Game/CharacterPart/Player/BP_BasePlayerChara` (`self.K2_GetPawn`)))
      (if (`/Game/CharacterPart/Player/BP_BasePlayerChara.CanMove` _asbp_base_player_chara_2)
        (`self.MoveToLocation` _cacheddestination)
        (`NiagaraFunctionLibrary.SpawnSystemAtLocation` (`self.FXCursor`) _cacheddestination))))
  (:`Completed`
    (goto _label)))

(event `InputAction|Dash`
  (params (Key :type "Key Structure"))
  (bind _playerchara (`self.PlayerChara`))
  (bind _playerchara_2 (`self.PlayerChara`))
  (bind _capsulecomponent (`Character.CapsuleComponent` (`GameplayStatics.GetPlayerCharacter` 0)))
  (:`Pressed`
    (if (> (`/Game/CharacterPart/Player/BP_BasePlayerChara.CurrentCool_Dodge` (`self.PlayerChara`)) 0.0)
      _
      (elif (not (`/Game/CharacterPart/Player/BP_BasePlayerChara.Skill_On` _playerchara))
        (set `/Game/CharacterPart/Player/BP_BasePlayerChara.Skill_On` true _playerchara)
        (set `/Game/CharacterPart/Player/BP_BasePlayerChara.CanMove` false _playerchara)
        (set `/Game/CharacterPart/Player/BP_BasePlayerChara.CurrentCool_Dodge` (`/Game/CharacterPart/Player/BP_BasePlayerChara.CoolTime_Dodge` _playerchara_2) _playerchara_2)
        (`self.StopMovement`)
        (bind _asbp_base_player_chara (cast `/Game/CharacterPart/Player/BP_BasePlayerChara` (`GameplayStatics.GetPlayerCharacter` 0)))
        (`/Game/CharacterPart/Player/BP_BasePlayerChara.Dodge` _asbp_base_player_chara)
        (bind _returnvalue (`self.K2_GetActorLocation` _asbp_base_player_chara))
        (bind (_returnvalue_x _returnvalue_y) (`KismetMathLibrary.BreakVector` (- (`SceneComponent.K2_GetComponentLocation` (`/Game/CharacterPart/Player/BP_BasePlayerChara.Cursor` _asbp_base_player_chara)) (`SceneComponent.K2_GetComponentLocation` (`Character.CapsuleComponent` _asbp_base_player_chara)))))
        (bind _returnvalue_2 (+ _returnvalue (* (`KismetMathLibrary.Normal` (`KismetMathLibrary.MakeVector` _returnvalue_x _returnvalue_y) 1.0) (800.0 800.0 0.0))))
        (bind (_outhit _returnvalue_3) (`KismetSystemLibrary.LineTraceSingle` _returnvalue _returnvalue_2 "TraceTypeQuery1"))
        (if _returnvalue_3
          (`KismetSystemLibrary.MoveComponentTo` _capsulecomponent (`.Location` (`GameplayStatics.BreakHitResult` _outhit)) (struct) false false 0.5 true)
          (else
            (`KismetSystemLibrary.MoveComponentTo` _capsulecomponent _returnvalue_2 (struct) false false 0.5 true)))))))

(fn `Follow`
  (params (Location :type "Vector Structure"))
  (bind _returnvalue (`self.K2_GetPawn`))
  (`Pawn.AddMovementInput` _returnvalue (`KismetMathLibrary.GetDirectionUnitVector` (`self.K2_GetActorLocation` _returnvalue) Location) 1.0 false))

(fn `Get Location Under Cursor`
  (returns (Location :type "Vector Structure") (Hit :type Boolean))
  (bind (_bblockinghit _binitialoverlap _time _distance _location) (`GameplayStatics.BreakHitResult` (`self.GetHitResultUnderCursorByChannel` "TraceTypeQuery3")))
  (return _location _bblockinghit))

(fn `MoveToLocation`
  (params (Location :type "Vector Structure"))
  (`AIBlueprintHelperLibrary.SimpleMoveToLocation` self Location))

(fn `UserConstructionScript`)