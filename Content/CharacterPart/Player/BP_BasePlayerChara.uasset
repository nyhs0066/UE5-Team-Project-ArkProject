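; Base player character that handles boss hit reactions, knockback and death, driving BP_RevenantAnim states and HP in BP_PlayerState.
; AnyDamage locks movement, clears skill state and casts the DamageType class to choose either a flinch or a Blowed launch away from the boss.
; Damage counts as a percentage of MaxHP.
; Tick detects zero HP or falls below the world, and Damaged spawns screen-projected damage widgets.
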(event `self.ReceiveBeginPlay`
  (bind _asbp_revenant_anim (cast `/Game/CharacterPart/Player/Anim/BP_RevenantAnim` (`SkeletalMeshComponent.GetAnimInstance` (`self.Mesh`))))
  (set `self.AnimBP` _asbp_revenant_anim)
  (bind _asbp_player_state (cast `/Game/Common/BP_PlayerState` (`GameplayStatics.GetPlayerState` 0)))
  (bind _output_get (set `self.BP_PlayerState` _asbp_player_state))
  (bind _playercharacterinformation (`/Game/Common/BP_PlayerState.PlayerCharacterInformation` _output_get))
  (`/Engine/EditorBlueprintResources/StandardMacros.IsValid` _playercharacterinformation
    (:`Is Valid`
      (set `/Game/Common/SaveGame/SG_Character.CurrentHP` (`/Game/Common/SaveGame/SG_Character.MaxHP` _playercharacterinformation) _playercharacterinformation))
    (:`Is Not Valid`
      (`KismetSystemLibrary.PrintString` "Is Not Valid"))))

(event `self.ReceiveActorBeginOverlap`
  (params (OtherActor :type "Actor Object Reference")))

(event `self.ReceiveTick`
  (params (DeltaSeconds :type "Float (single-precision)"))
  (bind _animbp (`self.AnimBP`))
  (bind _bp_playerstate (`self.BP_PlayerState`))
  (bind (_returnvalue_x _returnvalue_y _returnvalue_z) (`KismetMathLibrary.BreakVector` (`self.K2_GetActorLocation` self)))
  (bind _playercharacterinformation (`/Game/Common/BP_PlayerState.PlayerCharacterInformation` _bp_playerstate))
  (`/Engine/EditorBlueprintResources/StandardMacros.IsValid` _bp_playerstate
    (:`Is Valid`
      (`/Engine/EditorBlueprintResources/StandardMacros.IsValid` _playercharacterinformation
        (:`Is Valid`
          (if (<= (`/Game/Common/SaveGame/SG_Character.CurrentHP` _playercharacterinformation) 0.0)
            (set `/Game/Common/SaveGame/SG_Character.HPRecovery` 0.0 _playercharacterinformation)
            (`/Game/CharacterPart/Player/Anim/BP_RevenantAnim.ClearSkillState` _animbp)
            (set `/Game/CharacterPart/Player/Anim/BP_RevenantAnim.IsKnockDown` true _animbp)
            (set `self. IsAlive` false)
            (`PrimitiveComponent.SetCollisionObjectType` (`self.CapsuleComponent`) "ECC_GameTraceChannel2")
            (elif (<= _returnvalue_z -1000.0)
              (if (`self. IsAlive`)
                (set `self. IsAlive` false)
                (`KismetSystemLibrary.PrintString` "낙사")))))))))

(event `Dodge`)

(event `Damaged`
  (params (Damage :type "Float (double-precision)") (isCritical :type Boolean))
  (bind _returnvalue (`GameplayStatics.GetPlayerController` 0))
  ;[1 1 1] 데미지 이펙트 생성
  (bind _returnvalue_2 (`|CreateWidget` "/Game/UserInterface/Damage/W_Damage.W_Damage_C" _returnvalue))
  (`UserWidget.AddToViewport` _returnvalue_2 0)
  (`/Game/UserInterface/Damage/W_Damage.SetDamagedPosition` _returnvalue_2 (`PlayerController.ProjectWorldLocationToScreen` _returnvalue (`self.K2_GetActorLocation` self) false))
  (`/Game/UserInterface/Damage/W_Damage.Damage` _returnvalue_2 Damage isCritical))

(event `self.ReceiveAnyDamage`
  (params (Damage :type "Float (single-precision)") (DamageType :type "DamageType Object Reference") (InstigatedBy :type "Controller Object Reference") (DamageCauser :type "Actor Object Reference"))
  ;[1 1 1] 데미지 반응
  (set `self.CanMove` false)
  (set `self.Fire_On` true)
  (set `self.Skill_On` true)
  (`Controller.StopMovement` (`GameplayStatics.GetPlayerController` 0))
  (`/Game/CharacterPart/Player/Anim/BP_RevenantAnim.ClearSkillState` (`self.AnimBP`))
  (set `self.HitDamage` Damage)
  (set `self.Boss` DamageCauser)
  (cast `/Game/BossPart/DT/DT_Normal` DamageType
    (:`then`
      (`self.Hit_Normal`))
    (:`CastFailed`
      (cast `/Game/BossPart/DT/DT_Stampede` DamageType
        (:`then`
          (`self.Hit_Stampede`))
        (:`CastFailed`
          (cast `/Game/BossPart/DT/DT_AirStrike` DamageType
            (:`then`
              (`self.Hit_AirStrike`))
            (:`CastFailed`
              (cast `/Game/BossPart/DT/DT_ChargeAttack` DamageType
                (:`then`
                  (`self.Hit_ChargeAttack`))
                (:`CastFailed`
                  (cast `/Game/BossPart/DT/DT_TriAOE` DamageType
                    (:`then`
                      (`self.Hit_TriAOE`))
                    (:`CastFailed`
                      (cast `/Game/BossPart/DT/DT_JumpAttack` DamageType)
                      (`self.Hit_JumpAttack`))))))))))))

(event `Hit_Normal`
  ;[1 1 1] 데미지 반응
  (if (not (`/Game/CharacterPart/Player/Anim/BP_RevenantAnim.IsHit` (`self.AnimBP`)))
    (set `/Game/CharacterPart/Player/Anim/BP_RevenantAnim.IsHit` true (`self.AnimBP`))
    (bind _hitdamage (`self.Set Hit Damage` (`self.HitDamage`)))
    (`/Game/Common/BP_PlayerState.ReduceHP` (`self.BP_PlayerState`) _hitdamage)
    (`KismetSystemLibrary.PrintString` "노말어택 맞음 ㅠ")))

(event `Hit_Stampede`
  ;[1 1 1] 데미지 반응
  (`self.Blowed` (1000.0 1000.0 600.0))
  (bind _hitdamage (`self.Set Hit Damage` (`self.HitDamage`)))
  (`/Game/Common/BP_PlayerState.ReduceHP` (`self.BP_PlayerState`) _hitdamage))

(event `Hit_AirStrike`
  ;[1 1 1] 데미지 반응
  (if (not (`/Game/CharacterPart/Player/Anim/BP_RevenantAnim.IsHit` (`self.AnimBP`)))
    (set `/Game/CharacterPart/Player/Anim/BP_RevenantAnim.IsHit` true (`self.AnimBP`))
    (bind _hitdamage (`self.Set Hit Damage` (`self.HitDamage`)))
    (`/Game/Common/BP_PlayerState.ReduceHP` (`self.BP_PlayerState`) _hitdamage)
    (`KismetSystemLibrary.PrintString` "낙석맞음")))

(event `Hit_ChargeAttack`
  ;[1 1 1] 데미지 반응
  (`self.Blowed` (2000.0 2000.0 1500.0))
  (bind _hitdamage (`self.Set Hit Damage` (`self.HitDamage`)))
  (`/Game/Common/BP_PlayerState.ReduceHP` (`self.BP_PlayerState`) _hitdamage))

(event `Hit_TriAOE`
  ;[1 1 1] 데미지 반응
  (`self.Blowed` (3000.0 3000.0 2000.0))
  (bind _hitdamage (`self.Set Hit Damage` (`self.HitDamage`)))
  (`/Game/Common/BP_PlayerState.ReduceHP` (`self.BP_PlayerState`) _hitdamage))

(event `Hit_JumpAttack`
  ;[1 1 1] 데미지 반응
  (if (not (`/Game/CharacterPart/Player/Anim/BP_RevenantAnim.IsHit` (`self.AnimBP`)))
    (set `/Game/CharacterPart/Player/Anim/BP_RevenantAnim.IsHit` true (`self.AnimBP`))
    (bind _hitdamage (`self.Set Hit Damage` (`self.HitDamage`)))
    (`/Game/Common/BP_PlayerState.ReduceHP` (`self.BP_PlayerState`) _hitdamage)
    (`KismetSystemLibrary.PrintString` "점공맞음")))

(fn `Blowed`
  (params (Speed :type "Vector Structure"))
  (bind _charactermovement (`self.CharacterMovement`))
  (bind (_returnvalue_x _returnvalue_y) (`KismetMathLibrary.BreakVector` (- (`self.K2_GetActorLocation` self) (`self.K2_GetActorLocation` (`self.Boss`)))))
  (bind (_returnvalue_x_2 _returnvalue_y_2) (`KismetMathLibrary.BreakVector` (* (`KismetMathLibrary.Normal` (`KismetMathLibrary.MakeVector` _returnvalue_x _returnvalue_y) 1.0) (`KismetMathLibrary.MakeVector` Speed_X Speed_Y))))
  (if (not (`/Game/CharacterPart/Player/Anim/BP_RevenantAnim.IsKnockDown` (`self.AnimBP`)))
    (set `/Game/CharacterPart/Player/Anim/BP_RevenantAnim.IsKnockDown` true (`self.AnimBP`))
    (`PrimitiveComponent.SetCollisionObjectType` (`self.CapsuleComponent`) "ECC_GameTraceChannel2")
    (set `MovementComponent.Velocity` (`KismetMathLibrary.MakeVector` _returnvalue_x_2 _returnvalue_y_2 Speed_Z) _charactermovement)
    (`CharacterMovementComponent.SetMovementMode` _charactermovement "MOVE_Falling" 0)))

(fn `EffectOnOff`
  (params (EffectOn :type Boolean)))

(fn `SelectSkin`
  (params (MeshSkel :type "SkeletalMesh Object Reference")))

(fn `Set Hit Damage`
  (params (Damage :type "Float (double-precision)"))
  (returns (HitDamage :type "Float (double-precision)"))
  (return (* (/ Damage 100.0) (`/Game/Common/SaveGame/SG_Character.MaxHP` (`/Game/Common/BP_PlayerState.PlayerCharacterInformation` (`self.BP_PlayerState`))))))

(fn `UserConstructionScript`)