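; Player state Blueprint that owns the player's gameplay managers and in-game HUD.
; A one-time Initialize constructs UI, inventory, skill, quick-slot and status managers, creates W_InGameUI, then wires skill managers into its skillboard and quick slots.
; BeginPlay and Tick are empty; Initialize and Update are callable functions, with Update forwarding only to the skill manager.
; It also swaps or moves items between inventory and item quick-slot maps.
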(event `self.ReceiveBeginPlay`)

(fn `CreateManager`
  (`|ExecutionSequence`
    (:`then_0`
      (bind _returnvalue (`|GenericCreateObject` "/Game/UserInterface/InGameUI/BP_InGameUIManager.BP_InGameUIManager_C"))
      (set `self.InGameUIManager` _returnvalue))
    (:`then_1`
      (bind _returnvalue_2 (`|GenericCreateObject` "/Game/UserInterface/Inventory/BP_InventoryManager.BP_InventoryManager_C"))
      (set `self.InventoryManager` _returnvalue_2))
    (:`then_2`
      (bind _returnvalue_3 (`|GenericCreateObject` "/Game/UserInterface/Skill/BP_SkillManager.BP_SkillManager_C"))
      (set `self.SkillManager` _returnvalue_3))
    (:`then_3`
      (bind _returnvalue_4 (`|GenericCreateObject` "/Game/UserInterface/QuickSlot/BP_SkillQuickSlotsManager.BP_SkillQuickSlotsManager_C"))
      (set `self.SKillQuickSlotsManager` _returnvalue_4))
    (:`then_4`
      (bind _returnvalue_5 (`|GenericCreateObject` "/Game/UserInterface/QuickSlot/BP_ItemQuickSlotsManager.BP_ItemQuickSlotsManager_C"))
      (set `self.ItemQuickSlotsManager` _returnvalue_5))
    (:`then_5`
      (bind _returnvalue_6 (`|GenericCreateObject` "/Game/UserInterface/Status/BP_StatusManager.BP_StatusManager_C"))
      (set `self.StatusManager` _returnvalue_6))))

(fn `CreateUI`
  (bind _returnvalue (`|CreateWidget` "/Game/UserInterface/InGameUI/W_InGameUI.W_InGameUI_C"))
  (bind _output_get (set `self.InGameUI` _returnvalue))
  (`UserWidget.AddToViewport` _output_get 0))

(fn `Initialize`
  (if (not (`self.isInitialize`))
    (`self.CreateManager`)
    (`self.CreateUI`)
    (`self.SetUIVisible` true)
    (set `self.isInitialize` true)
    (`|ExecutionSequence`
      (:`then_0`
        (`self.InitializeManager`)
        (`self.InitializeWidget`)))))

(fn `InitializeManager`
  (`/Game/UserInterface/Skill/BP_SkillManager.Initialize` (`self.SkillManager`)))

(fn `InitializeWidget`
  (bind _ingameui (`self.InGameUI`))
  (`/Game/UserInterface/Skill/W_Skillboard.Initialize` (`/Game/UserInterface/InGameUI/W_InGameUI.W_Skillboard` _ingameui) (`self.SkillManager`))
  (`/Game/UserInterface/QuickSlot/W_SkillQuickSlots.SetSkillQuickSlotsManager` (`/Game/UserInterface/InGameUI/W_InGameUI.W_SkillQuickSlots` _ingameui) (`self.SKillQuickSlotsManager`)))

(fn `SetUIVisible`
  (params (Visible :type Boolean))
  (if Visible
    (`Widget.SetVisibility` (`self.InGameUI`) "Visible")
    (else
      (`Widget.SetVisibility` (`self.InGameUI`) "Hidden"))))

(fn `SwitchInvenSlotAndQuickSlot`
  (params (InventorySlotIndex :type Integer) (QuickSlotIndex :type Integer))
  (returns (Result :type Boolean))
  (locals (InventoryIndex :type Integer) (QuickIndex :type Integer) (isExistInventoryItem :type Boolean) (isExistQuickSlotItem :type Boolean) (TempQuickSlotItem :type "/Game/UserInterface/Inventory/BP_ItemSlot Object Reference") (TempInventoryItem :type "/Game/UserInterface/Inventory/BP_ItemSlot Object Reference"))
  (bind (_value _returnvalue) (`BlueprintMapLibrary.Map_Find` (`/Game/UserInterface/Inventory/BP_InventoryManager.Slots` (`self.InventoryManager`)) (`local.InventoryIndex`)))
  (bind (_value_2 _returnvalue_2) (`BlueprintMapLibrary.Map_Find` (`/Game/UserInterface/QuickSlot/BP_ItemQuickSlotsManager.Slots` (`self.ItemQuickSlotsManager`)) (`local.QuickIndex`)))
  (set `local.InventoryIndex` InventorySlotIndex)
  (set `local.QuickIndex` QuickSlotIndex)
  (`|ExecutionSequence`
    (:`then_0`
      (set `local.TempInventoryItem` _value)
      (set `local.isExistInventoryItem` _returnvalue))
    (:`then_1`
      (set `local.TempQuickSlotItem` _value_2)
      (set `local.isExistQuickSlotItem` _returnvalue_2))
    (:`then_2`
      (if (and (`local.isExistInventoryItem`) (`local.isExistQuickSlotItem`))
        (`BlueprintMapLibrary.Map_Add` (`/Game/UserInterface/Inventory/BP_InventoryManager.Slots` (`self.InventoryManager`)) (`local.InventoryIndex`) (`local.TempQuickSlotItem`))
        (`BlueprintMapLibrary.Map_Add` (`/Game/UserInterface/QuickSlot/BP_ItemQuickSlotsManager.Slots` (`self.ItemQuickSlotsManager`)) (`local.QuickIndex`) (`local.TempInventoryItem`))
        (return true)
        (else
          (`|ExecutionSequence`
            (:`then_0`
              (if (`local.isExistInventoryItem`)
                (`BlueprintMapLibrary.Map_Add` (`/Game/UserInterface/QuickSlot/BP_ItemQuickSlotsManager.Slots` (`self.ItemQuickSlotsManager`)) (`local.QuickIndex`) (`local.TempInventoryItem`))
                (`BlueprintMapLibrary.Map_Remove` (`/Game/UserInterface/Inventory/BP_InventoryManager.Slots` (`self.InventoryManager`)) (`local.InventoryIndex`))))
            (:`then_1`
              (if (`local.isExistQuickSlotItem`)
                (`BlueprintMapLibrary.Map_Add` (`/Game/UserInterface/Inventory/BP_InventoryManager.Slots` (`self.InventoryManager`)) (`local.InventoryIndex`) (`local.TempQuickSlotItem`))
                (`BlueprintMapLibrary.Map_Remove` (`/Game/UserInterface/QuickSlot/BP_ItemQuickSlotsManager.Slots` (`self.ItemQuickSlotsManager`)) (`local.QuickIndex`))))
            (:`then_2`
              (return true))))))))

(fn `Update`
  (params (DeltaTime :type "Float (double-precision)"))
  (`/Game/UserInterface/Skill/BP_SkillManager.Update` (`self.SkillManager`) DeltaTime))

(fn `UserConstructionScript`)