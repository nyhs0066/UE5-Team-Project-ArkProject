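; Map-part Blueprint for a half outer circle rim built from Geometry Collection floor and trim pieces that can be made to fall.
; FallingFloor turns on physics simulation for four Geometry Collection components (jungle trims, curved trim and plains floor block) when OnPhysicsSimul is false.
; The function does not set that flag itself, and the event graph and construction script are empty, so the collapse relies on an external call.
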(fn `Falling Floor`
  (if (not (`self.bOnPhysicsSimul`))
    (`|ExecutionSequence`
      (:`then_0`
        (`PrimitiveComponent.SetSimulatePhysics` (`self.GC_JungleTrim_1_GeometryCollectionComponent0`) true))
      (:`then_1`
        (`PrimitiveComponent.SetSimulatePhysics` (`self.GC_Plains_Floors_Block_0_GeometryCollectionComponent0`) true))
      (:`then_2`
        (`PrimitiveComponent.SetSimulatePhysics` (`self.GC_JungleTrim_0_GeometryCollectionComponent0`) true))
      (:`then_3`
        (`PrimitiveComponent.SetSimulatePhysics` (`self.GC_JungleTrimCurved_0_GeometryCollectionComponent0`) true)))))

(fn `UserConstructionScript`)