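; BP_HalfOuterCircleFloor_1 is a half outer circle floor map piece that can collapse under physics.
; On BeginPlay it gathers the static mesh components among SharedRoot's direct children into StaticMeshGroup and logs the count.
; Falling Floor enables physics on that group while OnPhysicsSimul is false, without changing the flag.
; Toggle Simulate Physics flips the flag and applies it to every mesh; nothing in this Blueprint calls either function.
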(event `self.ReceiveBeginPlay`
  (`self.MakeStaticMeshGroup` (`self.StaticMeshGroup`))
  (set `self.On Physics Simul` false))

(fn `Falling Floor`
  (if (not (`self.On Physics Simul`))
    (for _array_element (`self.StaticMeshGroup`)
      (`PrimitiveComponent.SetSimulatePhysics` _array_element true))))

(fn `MakeStaticMeshGroup`
  (params (Array :type "Array of StaticMeshComponent Object Reference (by ref)"))
  (for _array_element (`SceneComponent.GetChildrenComponents` (`self.SharedRoot`) false)
    (bind `_as스태틱_메시_컴포넌트` (cast `StaticMeshComponent` _array_element))
    (`KismetArrayLibrary.Array_Add` Array `_as스태틱_메시_컴포넌트`))
  (`KismetSystemLibrary.LogString` (`KismetStringLibrary.JoinStringArray` (`|MakeArray` "Static Mesh Length : " (`KismetStringLibrary.Conv_IntToString` (`KismetArrayLibrary.Array_Length` Array))) "")))

(fn `Toggle Simulate Physics`
  (bind _output_get (set `self.On Physics Simul` (not (`self.On Physics Simul`))))
  (for _array_element (`self.StaticMeshGroup`)
    (`PrimitiveComponent.SetSimulatePhysics` _array_element _output_get)))

(fn `UserConstructionScript`)