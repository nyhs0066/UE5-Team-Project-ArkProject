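; BP_ImpulseField is a Chaos field actor that applies a one-shot break-and-push impulse to physics objects when spawned or at level start.
; On BeginPlay it sizes its Sphere from SphereRadius and waits briefly.
; It then applies a radial-falloff external cluster strain field with no falloff, followed by a radial-vector linear velocity field.
; Both fields are centered on the Sphere, with separately configurable magnitudes.
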(event `self.ReceiveBeginPlay`
  (bind _sphere (`self.Sphere`))
  (bind _fieldsystemcomponent (`self.FieldSystemComponent`))
  (bind _returnvalue (`SceneComponent.K2_GetComponentLocation` _sphere))
  (`SphereComponent.SetSphereRadius` _sphere (`self.Sphere Radius`) true)
  (`KismetSystemLibrary.Delay` 0.2)
  (`FieldSystemComponent.ApplyPhysicsField` _fieldsystemcomponent true "Field_ExternalClusterStrain" null (`RadialFalloff.SetRadialFalloff` (`self.RadialFalloff`) (`self.Field Magnitude`) 0.0 1.0 0.0 (`self.Sphere Radius`) _returnvalue "Field_FallOff_None"))
  (`FieldSystemComponent.ApplyPhysicsField` _fieldsystemcomponent true "Field_LinearVelocity" null (`RadialVector.SetRadialVector` (`self.RadialVector`) (`self.Vector Magnitude`) _returnvalue)))

(event `self.ReceiveTick`
  (params (DeltaSeconds :type "Float (single-precision)")))

(fn `UserConstructionScript`)