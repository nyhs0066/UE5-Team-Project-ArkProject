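; BP_SkillSlot represents one skill slot, holding a skill's info, level, cooldown progress and skill actor.
; Getters expose SkillInfo fields such as name, icon, class, costs and Korean type labels, with per-level damage read from the skill's DataTable.
; A cooldown check reports true once CoolingTime reaches CoolTime or when none is set.
; Activate hands the slot to its BP_SkillBase actor and starts it, while Deactivate sets that actor's IsEnd to false.
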(fn `Activate`
  (set `self.isActivated` true)
  (bind _asbp_skill_base (cast `/Game/UserInterface/Skill/BP_SkillBase` (`self.SkillActor`)))
  (`/Engine/EditorBlueprintResources/StandardMacros.IsValid` _asbp_skill_base
    (:`Is Valid`
      (set `/Game/UserInterface/Skill/BP_SkillBase.SkillSlot` self _asbp_skill_base)
      (`/Game/UserInterface/Skill/BP_SkillBase.Activate` _asbp_skill_base))))

(fn `Deactivate`
  (bind _asbp_skill_base (cast `/Game/UserInterface/Skill/BP_SkillBase` (`self.SkillActor`)))
  (`/Engine/EditorBlueprintResources/StandardMacros.IsValid` _asbp_skill_base
    (:`Is Valid`
      (set `/Game/UserInterface/Skill/BP_SkillBase.isEnd` false _asbp_skill_base))))

(fn `GetClassReference`
  (returns (SkillClassRef :type "Actor Class Reference"))
  (bind (_skillinfo_id _skillinfo_name _skillinfo_classreference) (break `/Game/Common/Struct/S_SKillInfo` (`self.SkillInfo`)))
  (return _skillinfo_classreference))

(fn `GetCoolTime`
  (returns (CoolTime :type "Float (double-precision)"))
  (bind (_skillinfo_id _skillinfo_name _skillinfo_classreference _skillinfo_icon _skillinfo_cooltime) (break `/Game/Common/Struct/S_SKillInfo` (`self.SkillInfo`)))
  (return _skillinfo_cooltime))

(fn `GetDamagePercentage`
  (returns (Count :type Integer) (DamagePercentage :type "Float (double-precision)"))
  (bind (_skillinfo_id _skillinfo_name _skillinfo_classreference _skillinfo_icon _skillinfo_cooltime _skillinfo_type _skillinfo_damagetable) (break `/Game/Common/Struct/S_SKillInfo` (`self.SkillInfo`)))
  (bind _returnvalue (`|GetDataTableRow` _skillinfo_damagetable (`KismetStringLibrary.Conv_StringToName` (`KismetStringLibrary.Conv_IntToString` (`self.Level`))))
    (:`then`
      (bind (_level _count _damagepercentage) (break `/Game/Common/Struct/S_SkillDamageOfLevel` _returnvalue))
      (return _count _damagepercentage))))

(fn `GetIcon`
  (returns (Icon :type "Texture2D Object Reference"))
  (bind (_skillinfo_id _skillinfo_name _skillinfo_classreference _skillinfo_icon) (break `/Game/Common/Struct/S_SKillInfo` (`self.SkillInfo`)))
  (return _skillinfo_icon))

(fn `GetName`
  (returns (Name :type Text))
  (bind (_skillinfo_id _skillinfo_name) (break `/Game/Common/Struct/S_SKillInfo` (`self.SkillInfo`)))
  (return (`KismetTextLibrary.Conv_NameToText` _skillinfo_name)))

(fn `GetSkillCost`
  (returns (HPCost :type "Float (double-precision)") (MPCost :type "Float (double-precision)") (IdentityCost :type "Float (double-precision)"))
  (bind (_skillinfo_id _skillinfo_name _skillinfo_classreference _skillinfo_icon _skillinfo_cooltime _skillinfo_type _skillinfo_damagetable _skillinfo_description _skillinfo_ismovable _skillinfo_hpcost _skillinfo_mpcost _skillinfo_identitycost) (break `/Game/Common/Struct/S_SKillInfo` (`self.SkillInfo`)))
  (return _skillinfo_hpcost _skillinfo_mpcost _skillinfo_identitycost))

(fn `GetSkillInfo`
  (returns (SkillInfo :type "/Game/Common/Struct/S_SKillInfo Structure"))
  (bind _skillinfo_id (break `/Game/Common/Struct/S_SKillInfo` (`self.SkillInfo`)))
  (if (< _skillinfo_id 1)
    (return)
    (else
      (return (`self.SkillInfo`)))))

(fn `GetSkillType`
  (returns (NewParam :type "/Game/Common/Enum/E_SkillType Enum"))
  (bind (_skillinfo_id _skillinfo_name _skillinfo_classreference _skillinfo_icon _skillinfo_cooltime _skillinfo_type) (break `/Game/Common/Struct/S_SKillInfo` (`self.SkillInfo`)))
  (return _skillinfo_type))

(fn `GetSkillTypeText`
  (returns (SkillType :type Text))
  (bind (_skillinfo_id _skillinfo_name _skillinfo_classreference _skillinfo_icon _skillinfo_cooltime _skillinfo_type) (break `/Game/Common/Struct/S_SKillInfo` (`self.SkillInfo`)))
  (switch `/Game/Common/Enum/E_SkillType` _skillinfo_type
    (:`NewEnumerator0`
      (return "발동"))
    (:`NewEnumerator1`
      (return "홀딩"))
    (:`NewEnumerator2`
      (return "시전"))
    (:`NewEnumerator3`
      (return "설치"))))

(fn `isCoolDown`
  (returns (CoolDown :type Boolean))
  (bind (_skillinfo_id _skillinfo_name _skillinfo_classreference _skillinfo_icon _skillinfo_cooltime) (break `/Game/Common/Struct/S_SKillInfo` (`self.SkillInfo`)))
  (if (> _skillinfo_cooltime 0.0)
    (return (>= (`self.CoolingTime`) _skillinfo_cooltime))
    (else
      (return true))))