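; BP_SkillManager builds and maintains a character's list of skill slots, filtered by job class.
; Initialize reads DT_SkillInfo rows by incrementing numeric row name until one is missing, constructing a BP_SkillSlot for each matching job.
; SetSkillInfo copies the row data and ID into each slot and starts it at level one.
; Update adds the passed time to every slot's CoolingTime.
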(fn `Initialize`
  (params (CharacterInformation :type "/Game/Common/SaveGame/SG_Character Object Reference (by ref)"))
  (locals (isEmpty :type Boolean) (Index :type Integer :default 1))
  (while (not (`local.isEmpty`))
    (bind _returnvalue (`|GetDataTableRow` "/Game/Common/DataTable/DT_SkillInfo.DT_SkillInfo" (`KismetStringLibrary.Conv_StringToName` (`KismetStringLibrary.Conv_IntToString` (`local.Index`))))
      (:`then`
        (if (`|EnumEquality` (`/Game/Common/SaveGame/SG_Character.JobClass` CharacterInformation) (`.Job_41_B2DBC08D4F27FF9C3733E9B2390AE7C2` (break `/Game/Common/Struct/S_SKillInfo` _returnvalue)))
          (bind _returnvalue_2 (`|GenericCreateObject` self (`self.SkillSlotClassRef`)))
          (bind _asbp_skill_slot (cast `/Game/UserInterface/Skill/BP_SkillSlot` _returnvalue_2))
          (bind _return (`self.SetSkillInfo` _returnvalue _asbp_skill_slot))
          (`KismetArrayLibrary.Array_Add` (`self.SkillSlotArray`) _return)
          (set `local.Index` (+ (`local.Index`) 1))
          (else
            (set `local.Index` (+ (`local.Index`) 1)))))
      (:`RowNotFound`
        (set `local.isEmpty` true)))))

(fn `SetSkillInfo`
  (params (SrcInfo :type "/Game/Common/Struct/S_SKillInfo Structure") (TargetSlot :type "/Game/UserInterface/Skill/BP_SkillSlot Object Reference (by ref)"))
  (returns (Return :type "/Game/UserInterface/Skill/BP_SkillSlot Object Reference"))
  (bind _output_get (set `/Game/UserInterface/Skill/BP_SkillSlot.SkillInfo` SrcInfo TargetSlot))
  (set `/Game/UserInterface/Skill/BP_SkillSlot.ID` (`.ID_7_4997218E4775724981AAD6AE9558831B` (break `/Game/Common/Struct/S_SKillInfo` _output_get)) TargetSlot)
  (set `/Game/UserInterface/Skill/BP_SkillSlot.Level` 1 TargetSlot)
  (return TargetSlot))

(fn `Update`
  (params (Time :type "Float (double-precision) (by ref)"))
  (for _array_element (`self.SkillSlotArray`)
    (set `/Game/UserInterface/Skill/BP_SkillSlot.CoolingTime` (+ (`/Game/UserInterface/Skill/BP_SkillSlot.CoolingTime` _array_element) Time) _array_element)))