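; BP_SkillBase is a base skill actor that manages activation, deactivation and cooldown for its SkillSlot.
; Activate resets the slot's cooling time and calls OnActive, while Deactivate clears the slot's active flag, marks the skill ended and calls OnDeactive.
; Once ended, Tick accumulates cooling time on the slot and destroys the actor when the cooldown completes.
; SetMovable and UnlockMove only cast to the top-down controller, with no further effect.
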(event `self.ReceiveTick`
  (params (DeltaSeconds :type "Float (single-precision)"))
  (bind _skillslot (`self.SkillSlot`))
  (if (`self.isEnd`)
    (bind _output_get (set `/Game/UserInterface/Skill/BP_SkillSlot.CoolingTime` (+ (`/Game/UserInterface/Skill/BP_SkillSlot.CoolingTime` _skillslot) DeltaSeconds) _skillslot))
    (if (>= _output_get (`/Game/UserInterface/Skill/BP_SkillSlot.GetCoolTime` _skillslot))
      (`self.K2_DestroyActor`))))

(fn `Activate`
  (set `/Game/UserInterface/Skill/BP_SkillSlot.CoolingTime` 0.0 (`self.SkillSlot`))
  (`self.SetMovable`)
  (`self.OnActive`))

(fn `Deactivate`
  (set `/Game/UserInterface/Skill/BP_SkillSlot.isActivated` false (`self.SkillSlot`))
  (set `self.isEnd` true)
  (`self.UnlockMove`)
  (`self.OnDeactive`))

(fn `SetMovable`
  (cast `/Game/MapPart/TopDown/Blueprints/BP_TopDownController` (`GameplayStatics.GetPlayerController` 0)))

(fn `UnlockMove`
  (cast `/Game/MapPart/TopDown/Blueprints/BP_TopDownController` (`GameplayStatics.GetPlayerController` 0)))

(fn `UserConstructionScript`)