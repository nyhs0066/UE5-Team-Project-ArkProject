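; BP_Item is a world item actor that shows a floating name tag and can be picked up.
; On BeginPlay it looks up its ID in DT_ItemList to set name and meshes, then creates a W_NameTag viewport widget.
; A Delay on Tick throttles projecting the actor's location to screen to reposition the centered tag roughly every 0.2 seconds.
; Picked removes the tag and destroys the actor.
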(event `self.ReceiveBeginPlay`
  (`self.Update`)
  (`self.CreateNameTag`))

(event `self.ReceiveTick`
  (params (DeltaSeconds :type "Float (single-precision)"))
  (`KismetSystemLibrary.Delay` 0.2)
  (`self.UpdateNameTag`))

(fn `CreateNameTag`
  (bind _returnvalue (`|CreateWidget` (`self.NameTagClassRef`)))
  (bind _output_get (set `self.NameTag` _returnvalue))
  (bind _asw_name_tag (cast `/Game/UserInterface/Item/W_NameTag` _output_get))
  (`/Game/UserInterface/Item/W_NameTag.SetName` _asw_name_tag (`KismetStringLibrary.Conv_NameToString` (`self.Name`)))
  (`UserWidget.AddToViewport` _output_get 0))

(fn `Picked`
  (`Widget.RemoveFromParent` (`self.NameTag`))
  (`self.K2_DestroyActor`))

(fn `Update`
  (bind _returnvalue (`|GetDataTableRow` "/Game/DataTable/DT_ItemList.DT_ItemList" (`KismetStringLibrary.Conv_StringToName` (`KismetStringLibrary.Conv_IntToString` (`self.ID`))))
    (:`then`
      (set `self.Name` (`.Name_23_5DA12C1A4D385A599E3D21AC03C79361` (break `/Game/Common/Struct/S_Item` _returnvalue)))
      (`SkinnedMeshComponent.SetSkinnedAssetAndUpdate` (`self.SkeletalMesh`) (`.SkeletalMesh_42_A4D801FF40062142CFE3218CDE5432AD` (break `/Game/Common/Struct/S_Item` _returnvalue)) true)
      (`StaticMeshComponent.SetStaticMesh` (`self.StaticMesh`) (`.StaticMesh_45_8F931EB94332D52A8BE634B895AB5269` (break `/Game/Common/Struct/S_Item` _returnvalue))))))

(fn `UpdateNameTag`
  (bind _nametag (`self.NameTag`))
  (`UserWidget.SetPositionInViewport` _nametag (`PlayerController.ProjectWorldLocationToScreen` (`GameplayStatics.GetPlayerController` 0) (`self.K2_GetActorLocation`) false) true)
  (`UserWidget.SetAlignmentInViewport` _nametag (0.5 0.5)))

(fn `UserConstructionScript`)