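; BP_Potion_MP is an item Blueprint for a mana potion that restores part of the player's MP when used.
; On BeginPlay it binds a handler to the OnUseItem event.
; The handler casts player state 0 to BP_PlayerState and adds 30% of MaxMP to CurrentMP in PlayerCharacterInformation, clamped between zero and MaxMP.
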(event `self.ReceiveBeginPlay`
  (`parent.ReceiveBeginPlay`)
  (add `self.OnUseItem` (delegate `OnUsedItem`)))

(event `OnUsedItem`
  (bind _asbp_player_state (cast `/Game/Common/BP_PlayerState` (`GameplayStatics.GetPlayerState` 0)))
  (bind _playercharacterinformation (`/Game/Common/BP_PlayerState.PlayerCharacterInformation` _asbp_player_state))
  (bind _maxmp (`/Game/Common/SaveGame/SG_Character.MaxMP` _playercharacterinformation))
  (set `/Game/Common/SaveGame/SG_Character.CurrentMP` (`KismetMathLibrary.FClamp` (+ (`/Game/Common/SaveGame/SG_Character.CurrentMP` _playercharacterinformation) (* _maxmp 0.3)) 0.0 _maxmp) _playercharacterinformation))

(fn `UserConstructionScript`
  (`parent.UserConstructionScript`))