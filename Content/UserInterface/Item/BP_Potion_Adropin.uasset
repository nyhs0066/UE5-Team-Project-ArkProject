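; Adrenaline-style potion item (Adropin) that gives the player a temporary attack speed and movement speed boost.
; BeginPlay binds UsedItem to OnUseItem, which adds a fixed bonus to both stats in player 0's BP_PlayerState character information.
; Tick accumulates DurationCounter regardless of use, then subtracts the same bonus once when Duration is reached and sets IsFinish.
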(event `self.ReceiveBeginPlay`
  (`parent.ReceiveBeginPlay`)
  (add `self.OnUseItem` (delegate `UsedItem`)))

(event `UsedItem`
  (bind _asbp_player_state (cast `/Game/Common/BP_PlayerState` (`GameplayStatics.GetPlayerState` 0)))
  (bind _playercharacterinformation (`/Game/Common/BP_PlayerState.PlayerCharacterInformation` _asbp_player_state))
  (set `/Game/Common/SaveGame/SG_Character.AttackSpeed` (+ (`/Game/Common/SaveGame/SG_Character.AttackSpeed` _playercharacterinformation) 0.5) _playercharacterinformation)
  (set `/Game/Common/SaveGame/SG_Character.MovementSpeed` (+ (`/Game/Common/SaveGame/SG_Character.MovementSpeed` _playercharacterinformation) 0.5) _playercharacterinformation))

(event `self.ReceiveTick`
  (params (DeltaSeconds :type "Float (single-precision)"))
  (`parent.ReceiveTick` DeltaSeconds)
  (if (not (`self.isFinish`))
    (bind _output_get (set `self.DurationCounter` (+ (`self.DurationCounter`) DeltaSeconds)))
    (if (>= _output_get (`self.Duration`))
      (set `self.isFinish` true)
      (bind _asbp_player_state (cast `/Game/Common/BP_PlayerState` (`GameplayStatics.GetPlayerState` 0)))
      (bind _playercharacterinformation (`/Game/Common/BP_PlayerState.PlayerCharacterInformation` _asbp_player_state))
      (set `/Game/Common/SaveGame/SG_Character.AttackSpeed` (- (`/Game/Common/SaveGame/SG_Character.AttackSpeed` _playercharacterinformation) 0.5) _playercharacterinformation)
      (set `/Game/Common/SaveGame/SG_Character.MovementSpeed` (- (`/Game/Common/SaveGame/SG_Character.MovementSpeed` _playercharacterinformation) 0.5) _playercharacterinformation))))

(fn `UserConstructionScript`
  (`parent.UserConstructionScript`))