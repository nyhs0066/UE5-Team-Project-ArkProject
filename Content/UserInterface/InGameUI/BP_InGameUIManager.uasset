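; In-game UI manager that coordinates item transfers between the inventory and the item quick slots.
; AddItemToInventory forwards items to InventoryManager, calling Picked on the item and returning false when AddItem returns false.
; SwitchInventorySlotAndQuickSlot caches both slot entries, then swaps them, or moves the only occupied one, by editing each manager's Slots map.
; Slot switches end by calling UpdateUI, which is an empty stub here.
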(fn `AddItemToInventory`
  (params (TargetItem :type "/Game/UserInterface/Item/BP_Item Object Reference"))
  (returns (Failed :type Boolean))
  (bind _failed (`/Game/UserInterface/Inventory/BP_InventoryManager.AddItem` (`self.InventoryManager`) TargetItem))
  (if (not _failed)
    (`/Game/UserInterface/Item/BP_Item.Picked` TargetItem)
    (return false)
    (else
      (return true))))

(fn `SwitchInventorySlotAndQuickSlot`
  (params (InventorySlotIndex :type Integer) (QuickSlotIndex :type Integer))
  (returns (Result :type Boolean))
  (locals (InventoryIndex :type Integer) (QuickIndex :type Integer) (TempInventoryItem :type "/Game/UserInterface/Inventory/BP_ItemSlot Object Reference") (isExistInventoryItem :type Boolean) (TempQuickSlotItem :type "/Game/UserInterface/Inventory/BP_ItemSlot Object Reference") (isExistQuickSlotItem :type Boolean))
  (bind (_value _returnvalue) (`BlueprintMapLibrary.Map_Find` (`/Game/UserInterface/Inventory/BP_InventoryManager.Slots` (`self.InventoryManager`)) (`local.InventoryIndex`)))
  (bind (_value_2 _returnvalue_2) (`BlueprintMapLibrary.Map_Find` (`/Game/UserInterface/QuickSlot/BP_ItemQuickSlotsManager.Slots` (`self.ItemQuickSlotsManager`)) (`local.QuickIndex`)))
  (set `local.InventoryIndex` InventorySlotIndex)
  (set `local.QuickIndex` QuickSlotIndex)
  (`|ExecutionSequence`
    (:`then_0`
      (set `local.TempInventoryItem` _value)
      (set `local.isExistInventoryItem` _returnvalue))
    (:`then_1`
      (set `local.TempQuickSlotItem` _value_2)
      (set `local.isExistQuickSlotItem` _returnvalue_2))
    (:`then_2`
      (if (and (`local.isExistInventoryItem`) (`local.isExistQuickSlotItem`))
        (`BlueprintMapLibrary.Map_Add` (`/Game/UserInterface/Inventory/BP_InventoryManager.Slots` (`self.InventoryManager`)) (`local.InventoryIndex`) (`local.TempQuickSlotItem`))
        (`BlueprintMapLibrary.Map_Add` (`/Game/UserInterface/QuickSlot/BP_ItemQuickSlotsManager.Slots` (`self.ItemQuickSlotsManager`)) (`local.QuickIndex`) (`local.TempInventoryItem`))
        (`self.UpdateUI`)
        (return true)
        (else
          (`|ExecutionSequence`
            (:`then_0`
              (if (`local.isExistInventoryItem`)
                (`BlueprintMapLibrary.Map_Add` (`/Game/UserInterface/QuickSlot/BP_ItemQuickSlotsManager.Slots` (`self.ItemQuickSlotsManager`)) (`local.QuickIndex`) (`local.TempInventoryItem`))
                (`BlueprintMapLibrary.Map_Remove` (`/Game/UserInterface/Inventory/BP_InventoryManager.Slots` (`self.InventoryManager`)) (`local.InventoryIndex`))))
            (:`then_1`
              (if (`local.isExistQuickSlotItem`)
                (`BlueprintMapLibrary.Map_Add` (`/Game/UserInterface/Inventory/BP_InventoryManager.Slots` (`self.InventoryManager`)) (`local.InventoryIndex`) (`local.TempQuickSlotItem`))
                (`BlueprintMapLibrary.Map_Remove` (`/Game/UserInterface/QuickSlot/BP_ItemQuickSlotsManager.Slots` (`self.ItemQuickSlotsManager`)) (`local.QuickIndex`))))
            (:`then_2`
              (`self.UpdateUI`)
              (return true))))))))

(fn `UpdateUI`)