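; BP_SoundOption is a data holder for sound settings in the save options, covering global, effect and BGM channels.
; It stores a volume and a play setting for each of the three channels.
; SetVolume and SetPlay write these values, and GetVolume and GetPlay return them, with no further logic or audio application in the asset.
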(fn `GetPlay`
  (returns (GlobalPlay :type Boolean) (EffectPlay :type Boolean) (BGMPlay :type Boolean))
  (return (`self.GlobalPlay`) (`self.EffectPlay`) (`self.BGMPlay`)))

(fn `GetVolume`
  (returns (GlobalVolume :type Integer) (EffectVolume :type Integer) (BGMVolume :type Integer))
  (return (`self.GlobalVolume`) (`self.EffectVolume`) (`self.BGMVolume`)))

(fn `SetPlay`
  (params (Global :type Boolean) (Effect :type Boolean) (BGM :type Boolean))
  (set `self.GlobalPlay` Global)
  (set `self.EffectPlay` Effect)
  (set `self.BGMPlay` BGM))

(fn `SetVolume`
  (params (GlobalVolume :type Integer) (EffectVolume :type Integer) (BGMVolume :type Integer))
  (set `self.GlobalVolume` GlobalVolume)
  (set `self.EffectVolume` EffectVolume)
  (set `self.BGMVolume` BGMVolume))