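; Manages the player's skill quick slots as a map from slot index to skill info, with lookup by index.
; Swapping exchanges two entries or moves one into an empty slot.
; Adding replaces the target entry, first removing the index reported by the duplicate-ID check, which loops 1 to 8 but always reads key 0.
; A separate query reports whether any slotted skill is activated.
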(fn `AddSkillToSlot`
  (params (TargetIndex :type Integer) (TargetSlot :type "/Game/UserInterface/Skill/BP_SkillSlot Object Reference (by ref)"))
  (locals (SrcIndex :type Integer))
  (bind (_result _duplicatedindex) (`self.isDuplicatedSkill` TargetSlot))
  (bind _srcindex (`local.SrcIndex`))
  (set `local.SrcIndex` TargetIndex)
  (if (not _result)
    (if (`.ReturnValue` (`BlueprintMapLibrary.Map_Find` (`self.Slots`) (`local.SrcIndex`)))
      (`BlueprintMapLibrary.Map_Remove` (`self.Slots`) _srcindex))
    (`BlueprintMapLibrary.Map_Add` (`self.Slots`) _srcindex TargetSlot)
    (else
      (`BlueprintMapLibrary.Map_Remove` (`self.Slots`) _duplicatedindex)
      (`BlueprintMapLibrary.Map_Add` (`self.Slots`) (`local.SrcIndex`) TargetSlot))))

(fn `GetSlot`
  (params (Index :type Integer))
  (returns (Slot :type "/Game/UserInterface/Skill/BP_SkillSlot Object Reference") (isFind :type Boolean))
  (bind (_value _returnvalue) (`BlueprintMapLibrary.Map_Find` (`self.Slots`) Index))
  (return _value _returnvalue))

(fn `isActivatedAnySkill`
  (returns (Return :type Boolean))
  (bind _values (`BlueprintMapLibrary.Map_Values` (`self.Slots`)))
  (for _array_element _values
    (if (`/Game/UserInterface/Skill/BP_SkillSlot.isActivated` _array_element)
      (return true)))
  (return false))

(fn `isDuplicatedSkill`
  (params (SrcInfo :type "/Game/UserInterface/Skill/BP_SkillSlot Object Reference"))
  (returns (Result :type Boolean) (DuplicatedIndex :type Integer))
  (bind (_value _returnvalue) (`BlueprintMapLibrary.Map_Find` (`self.Slots`)))
  (for _index (range 1 9)
    (if _returnvalue
      (if (== (`/Game/UserInterface/Skill/BP_SkillSlot.ID` _value) (`/Game/UserInterface/Skill/BP_SkillSlot.ID` SrcInfo))
        (return true _index))))
  (return false 0))

(fn `SwapSlot`
  (params (SrcIndexA :type "Integer (by ref)") (SrcIndexB :type "Integer (by ref)"))
  (locals (IndexA :type Integer) (IndexB :type Integer) (isExistA :type Boolean) (isExistB :type Boolean) (TempA :type "/Game/UserInterface/Skill/BP_SkillSlot Object Reference") (TempB :type "/Game/UserInterface/Skill/BP_SkillSlot Object Reference"))
  (bind _slots (`self.Slots`))
  (if (!= SrcIndexA SrcIndexB)
    (bind _output_get (set `local.IndexA` SrcIndexA))
    (bind _output_get_2 (set `local.IndexB` SrcIndexB))
    (bind (_value _returnvalue) (`BlueprintMapLibrary.Map_Find` _slots _output_get))
    (bind _output_get_3 (set `local.isExistA` _returnvalue))
    (bind (_value_2 _returnvalue_2) (`BlueprintMapLibrary.Map_Find` _slots _output_get_2))
    (bind _output_get_4 (set `local.isExistB` _returnvalue_2))
    (set `local.TempA` _value)
    (set `local.TempB` _value_2)
    (if (and _output_get_4 _output_get_3)
      ;[1 1 1] Change both.
      (`BlueprintMapLibrary.Map_Add` (`self.Slots`) (`local.IndexA`) (`local.TempB`))
      (`BlueprintMapLibrary.Map_Add` (`self.Slots`) (`local.IndexB`) (`local.TempA`))
      (else
        ;[1 1 1] Change Either or Neither
        (`|ExecutionSequence`
          (:`then_0`
            (if (`local.isExistA`)
              (`BlueprintMapLibrary.Map_Add` (`self.Slots`) (`local.IndexB`) (`local.TempA`))
              (`BlueprintMapLibrary.Map_Remove` (`self.Slots`) (`local.IndexA`))))
          (:`then_1`
            (if (`local.isExistB`)
              (`BlueprintMapLibrary.Map_Add` (`self.Slots`) (`local.IndexA`) (`local.TempB`))
              (`BlueprintMapLibrary.Map_Remove` (`self.Slots`) (`local.IndexB`)))))))))