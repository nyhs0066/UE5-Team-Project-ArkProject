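; Quick slot manager that keeps a map of slot indices to BP_ItemSlot objects and handles stacking, swapping and using items.
; AddItem builds slot data from DT_ItemList, increments the count of a matching ID in slots 1–8, and returns true when nothing matches.
; One item type is excluded from matching.
; SwapSlot also supports moves into empty slots, and UseItem delegates to the slot object.
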(fn `AddItem`
  (params (SrcItem :type "/Game/UserInterface/Item/BP_Item Object Reference"))
  (returns (Failed :type Boolean))
  (bind _result (`self.ConvertToSlotData` SrcItem))
  (bind (_find _index) (`self.GetSlotIndex` _result))
  (if _find
    (`self.AddItemToSlot` _index)
    (return false)
    (else
      (return true))))

(fn `AddItemToSlot`
  (params (SrcIndex :type Integer))
  (bind (_value _returnvalue) (`BlueprintMapLibrary.Map_Find` (`self.Slots`) SrcIndex))
  (if _returnvalue
    (set `/Game/UserInterface/Inventory/BP_ItemSlot.Count` (+ (`/Game/UserInterface/Inventory/BP_ItemSlot.Count` _value) 1) _value)))

(fn `ConvertToSlotData`
  (params (SrcItem :type "/Game/UserInterface/Item/BP_Item Object Reference"))
  (returns (Result :type "/Game/UserInterface/Inventory/BP_ItemSlot Object Reference"))
  (locals (TargetItem :type "/Game/UserInterface/Item/BP_Item Object Reference") (SlotData :type "/Game/UserInterface/Inventory/BP_ItemSlot Object Reference"))
  (bind _output_get (set `local.TargetItem` SrcItem))
  (bind _returnvalue (`|GetDataTableRow` "/Game/Common/DataTable/DT_ItemList.DT_ItemList" (`KismetStringLibrary.Conv_StringToName` (`KismetStringLibrary.Conv_IntToString` (`/Game/UserInterface/Item/BP_Item.ID` _output_get))))
    (:`then`
      (bind _returnvalue_2 (`|GenericCreateObject` "/Game/UserInterface/Inventory/BP_ItemSlot.BP_ItemSlot_C"))
      (bind _output_get_2 (set `local.SlotData` _returnvalue_2))
      (bind (_id _name _skeletalmesh _icon _type) (break `/Game/Common/Struct/S_Item` _returnvalue))
      (set `/Game/UserInterface/Inventory/BP_ItemSlot.ID` _id _output_get_2)
      (set `/Game/UserInterface/Inventory/BP_ItemSlot.Type` _type _output_get_2)
      (return _output_get_2))))

(fn `GetSlotIndex`
  (params (SrcItem :type "/Game/UserInterface/Inventory/BP_ItemSlot Object Reference"))
  (returns (Find :type Boolean) (Index :type Integer))
  (locals (Target :type "/Game/UserInterface/Inventory/BP_ItemSlot Object Reference"))
  (bind _output_get (set `local.Target` SrcItem))
  (if (`|EnumInequality` (`/Game/UserInterface/Inventory/BP_ItemSlot.Type` _output_get) "NewEnumerator0")
    (for _index (range 1 9)
      (bind (_value _returnvalue) (`BlueprintMapLibrary.Map_Find` (`self.Slots`) _index))
      (if _returnvalue
        (if (== (`/Game/UserInterface/Inventory/BP_ItemSlot.ID` _value) (`/Game/UserInterface/Inventory/BP_ItemSlot.ID` (`local.Target`)))
          (return true _index))))
    (else
      (return false 0))))

(fn `SwapSlot`
  (params (SrcIndex1 :type Integer) (SrcIndex2 :type Integer))
  (locals (IndexA :type Integer) (IndexB :type Integer) (isExistA :type Boolean) (isExistB :type Boolean) (TempA :type "/Game/UserInterface/Inventory/BP_ItemSlot Object Reference") (TempB :type "/Game/UserInterface/Inventory/BP_ItemSlot Object Reference"))
  (bind _slots (`self.Slots`))
  (bind (_value _returnvalue) (`BlueprintMapLibrary.Map_Find` _slots (`local.IndexB`)))
  (bind (_value_2 _returnvalue_2) (`BlueprintMapLibrary.Map_Find` _slots (`local.IndexA`)))
  (if (!= SrcIndex1 SrcIndex2)
    (set `local.IndexA` SrcIndex1)
    (set `local.IndexB` SrcIndex2)
    (bind _output_get (set `local.isExistA` _returnvalue_2))
    (bind _output_get_2 (set `local.isExistB` _returnvalue))
    (set `local.TempA` _value_2)
    (set `local.TempB` _value)
    (if (and _output_get_2 _output_get)
      ;[1 1 1] Change both.
      (`BlueprintMapLibrary.Map_Add` (`self.Slots`) (`local.IndexA`) (`local.TempB`))
      (`BlueprintMapLibrary.Map_Add` (`self.Slots`) (`local.IndexB`) (`local.TempA`))
      (else
        ;[1 1 1] Change Either or Neither
        (`|ExecutionSequence`
          (:`then_0`
            (if (`local.isExistA`)
              (`BlueprintMapLibrary.Map_Add` (`self.Slots`) (`local.IndexB`) (`local.TempA`))
              (`BlueprintMapLibrary.Map_Remove` (`self.Slots`) (`local.IndexA`))))
          (:`then_1`
            (if (`local.isExistB`)
              (`BlueprintMapLibrary.Map_Add` (`self.Slots`) (`local.IndexA`) (`local.TempB`))
              (`BlueprintMapLibrary.Map_Remove` (`self.Slots`) (`local.IndexB`)))))))))

(fn `UseItem`
  (params (Index :type Integer))
  (bind (_value _returnvalue) (`BlueprintMapLibrary.Map_Find` (`self.Slots`) Index))
  (if _returnvalue
    (`/Game/UserInterface/Inventory/BP_ItemSlot.UseItem` _value)))