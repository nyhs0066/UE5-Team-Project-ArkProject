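; Inventory manager that stores item slots in an index-keyed map sized by rows times columns.
; AddItem builds a BP_ItemSlot from the item's DT_ItemList row, picks an index, then inserts it or increments the count.
; Equipment-type items (presumably NewEnumerator0) take the first empty slot, while others stack on a matching ID or fall back to the first gap.
; Also provides slot lookup, removal and swapping, including moves into empty slots.
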(fn `AddItem`
  (params (SrcItem :type "/Game/UserInterface/Item/BP_Item Object Reference"))
  (returns (Failed :type Boolean))
  (bind _resultitemslot (`self.ConvertToSlotData` SrcItem))
  (bind (_isfull _ispiled _dstindex) (`self.GetSlotIndex` _resultitemslot))
  (bind _failed (`self.AddItemToSlot` _isfull _ispiled _dstindex _resultitemslot))
  (return _failed))

(fn `AddItemToSlot`
  (params (isFull :type Boolean) (isPiled :type Boolean) (TargetIndex :type Integer) (TargetItem :type "/Game/UserInterface/Inventory/BP_ItemSlot Object Reference"))
  (returns (Failed :type Boolean))
  (bind (_value _returnvalue) (`BlueprintMapLibrary.Map_Find` (`self.Slots`) TargetIndex))
  (if (not isFull)
    (if (not isPiled)
      (`BlueprintMapLibrary.Map_Add` (`self.Slots`) TargetIndex TargetItem :!label _label)
      (elif (not _returnvalue)
        (goto _label)
        (else
          _)))
    (set `/Game/UserInterface/Inventory/BP_ItemSlot.Count` (+ (`/Game/UserInterface/Inventory/BP_ItemSlot.Count` _value) 1) _value)
    (set `/Game/UserInterface/Inventory/BP_ItemSlot.CurrentPosition` TargetIndex _value)
    (return false)
    (else
      (return true))))

(fn `ConvertToSlotData`
  (params (SrcItem :type "/Game/UserInterface/Item/BP_Item Object Reference"))
  (returns (ResultItemSlot :type "/Game/UserInterface/Inventory/BP_ItemSlot Object Reference"))
  (locals (TargetItem :type "/Game/UserInterface/Item/BP_Item Object Reference") (SlotData :type "/Game/UserInterface/Inventory/BP_ItemSlot Object Reference"))
  (bind _output_get (set `local.TargetItem` SrcItem))
  (bind _returnvalue (`|GetDataTableRow` "/Game/DataTable/DT_ItemList.DT_ItemList" (`KismetStringLibrary.Conv_StringToName` (`KismetStringLibrary.Conv_IntToString` (`/Game/UserInterface/Item/BP_Item.ID` _output_get))))
    (:`then`
      (bind _returnvalue_2 (`|GenericCreateObject` "/Game/UserInterface/Inventory/BP_ItemSlot.BP_ItemSlot_C"))
      (bind _output_get_2 (set `local.SlotData` _returnvalue_2))
      (bind (_id _name _skeletalmesh _icon _type) (break `/Game/Common/Struct/S_Item` _returnvalue))
      (set `/Game/UserInterface/Inventory/BP_ItemSlot.ID` _id _output_get_2)
      (set `/Game/UserInterface/Inventory/BP_ItemSlot.Type` _type _output_get_2)
      (return _output_get_2))))

(fn `GetItemSlot`
  (params (TargetIndex :type Integer))
  (returns (ItemSlot :type "/Game/UserInterface/Inventory/BP_ItemSlot Object Reference") (isFind :type Boolean))
  (bind (_value _returnvalue) (`BlueprintMapLibrary.Map_Find` (`self.Slots`) TargetIndex))
  (return _value _returnvalue))

(fn `GetSlotIndex`
  (params (SrcItemSlot :type "/Game/UserInterface/Inventory/BP_ItemSlot Object Reference"))
  (returns (isFull :type Boolean) (isPiled :type Boolean) (DstIndex :type Integer))
  (locals (Target :type "/Game/UserInterface/Inventory/BP_ItemSlot Object Reference") (CurrentPos :type Integer) (MaxSlotsCount :type Integer) (isFind :type Boolean) (EmptyPos :type Integer))
  (bind _currentpos (`local.CurrentPos`))
  (bind _currentpos_2 (`local.CurrentPos`))
  (bind (_value _returnvalue) (`BlueprintMapLibrary.Map_Find` (`self.Slots`) (`local.CurrentPos`)))
  (bind _output_get (set `local.Target` SrcItemSlot))
  (set `local.MaxSlotsCount` (* (`self.SlotRow`) (`self.SlotColumn`)))
  (if (`|EnumEquality` (`/Game/UserInterface/Inventory/BP_ItemSlot.Type` _output_get) "NewEnumerator0")
    ;[1 1 1] Search for Equipment.
    (while true
      (if (not (`.ReturnValue` (`BlueprintMapLibrary.Map_Find` (`self.Slots`) (`local.CurrentPos`))))
        (return false false (`local.CurrentPos`))
        (else
          (set `local.CurrentPos` (+ _currentpos_2 1))
          (if (>= _currentpos_2 (`local.MaxSlotsCount`))
            (return true false 0)))))
    (else
      ;[1 1 1] Search for Others.
      (while true
        (if (not _returnvalue)
          ;;[1 1 1] Search First Empty Slot Index
          (if (not (`local.isFind`))
            (set `local.isFind` true)
            (set `local.EmptyPos` (`local.CurrentPos`)))
          (else
            ;[1 1 1] Find Piled Item. Return Current Position If Founded, Eles Search Continue.
            (if (!= (`/Game/UserInterface/Inventory/BP_ItemSlot.ID` _value) (`/Game/UserInterface/Inventory/BP_ItemSlot.ID` (`local.Target`)))
              _
              (else
                (return false true (`local.CurrentPos`))))))
        (set `local.CurrentPos` (+ _currentpos 1))
        (if (>= _currentpos (`local.MaxSlotsCount`))
          (return false true (`local.EmptyPos`)))))))

(fn `RemoveItem`
  (params (TargetIndex :type Integer))
  (`BlueprintMapLibrary.Map_Remove` (`self.Slots`) TargetIndex))

(fn `SwapSlot`
  (params (FirstSrcIndex :type Integer) (SecondSrcIndex :type Integer))
  (locals (isExistA :type Boolean) (isExistB :type Boolean) (IndexA :type Integer) (IndexB :type Integer) (TempA :type "/Game/UserInterface/Inventory/BP_ItemSlot Object Reference") (TempB :type "/Game/UserInterface/Inventory/BP_ItemSlot Object Reference"))
  (bind _slots (`self.Slots`))
  (bind (_value _returnvalue) (`BlueprintMapLibrary.Map_Find` _slots (`local.IndexA`)))
  (bind (_value_2 _returnvalue_2) (`BlueprintMapLibrary.Map_Find` _slots (`local.IndexB`)))
  (if (!= FirstSrcIndex SecondSrcIndex)
    (set `local.IndexA` FirstSrcIndex)
    (set `local.IndexB` SecondSrcIndex)
    (bind _output_get (set `local.isExistA` _returnvalue))
    (bind _output_get_2 (set `local.isExistB` _returnvalue_2))
    (set `local.TempA` _value)
    (set `local.TempB` _value_2)
    (if (and _output_get_2 _output_get)
      ;[1 1 1] Change both.
      (`BlueprintMapLibrary.Map_Add` (`self.Slots`) (`local.IndexA`) (`local.TempB`))
      (`BlueprintMapLibrary.Map_Add` (`self.Slots`) (`local.IndexB`) (`local.TempA`))
      (else
        ;[1 1 1] Change Either or Neither
        (`|ExecutionSequence`
          (:`then_0`
            (if (`local.isExistA`)
              (`BlueprintMapLibrary.Map_Add` (`self.Slots`) (`local.IndexB`) (`local.TempA`))
              (`BlueprintMapLibrary.Map_Remove` (`self.Slots`) (`local.IndexA`))))
          (:`then_1`
            (if (`local.isExistB`)
              (`BlueprintMapLibrary.Map_Add` (`self.Slots`) (`local.IndexA`) (`local.TempB`))
              (`BlueprintMapLibrary.Map_Remove` (`self.Slots`) (`local.IndexB`)))))))))