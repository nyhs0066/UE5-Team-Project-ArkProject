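; Inventory slot that holds an item's ID, position, count, activation state and cooldown data.
; It looks up the icon in DT_ItemList using the ID as row name, while class reference and cooldown length come from its cached ItemInfo.
; Using the item flags the slot as activated and hands a self-reference to its BP_Item actor.
; The cooldown check tests whether CoolingTime has reached the item's CoolTime.
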(fn `ClearData`
  (set `self.ID` -3)
  (set `self.CurrentPosition` -1)
  (set `self.Count` 0))

(fn `GetClassReference`
  (returns (ItemClassRef :type "Actor Class Reference"))
  (bind (_iteminfo_id _iteminfo_name _iteminfo_skeletalmesh _iteminfo_icon _iteminfo_type _iteminfo_description _iteminfo_staticmesh _iteminfo_cooltime _iteminfo_classref) (break `/Game/Common/Struct/S_Item` (`self.ItemInfo`)))
  (return _iteminfo_classref))

(fn `GetCoolTime`
  (returns (CoolTime :type "Float (double-precision)"))
  (bind (_iteminfo_id _iteminfo_name _iteminfo_skeletalmesh _iteminfo_icon _iteminfo_type _iteminfo_description _iteminfo_staticmesh _iteminfo_cooltime) (break `/Game/Common/Struct/S_Item` (`self.ItemInfo`)))
  (return _iteminfo_cooltime))

(fn `GetIcon`
  (returns (Icon :type "Texture2D Object Reference"))
  (bind _returnvalue (`|GetDataTableRow` "/Game/DataTable/DT_ItemList.DT_ItemList" (`KismetStringLibrary.Conv_StringToName` (`KismetStringLibrary.Conv_IntToString` (`self.ID`))))
    (:`then`
      (return (`.Icon_28_D34BE65346F21C744ACB7BBFEE4A676B` (break `/Game/Common/Struct/S_Item` _returnvalue))))))

(fn `isCoolDown`
  (returns (CoolDown :type Boolean))
  (bind (_iteminfo_id _iteminfo_name _iteminfo_skeletalmesh _iteminfo_icon _iteminfo_type _iteminfo_description _iteminfo_staticmesh _iteminfo_cooltime) (break `/Game/Common/Struct/S_Item` (`self.ItemInfo`)))
  (return (>= (`self.CoolingTime`) _iteminfo_cooltime)))

(fn `UseItem`
  (set `self.isActivated` true)
  (bind _asbp_item (cast `/Game/UserInterface/Item/BP_Item` (`self.ItemActor`)))
  (`/Engine/EditorBlueprintResources/StandardMacros.IsValid` _asbp_item
    (:`Is Valid`
      (set `/Game/UserInterface/Item/BP_Item.ItemSlot` self _asbp_item))))