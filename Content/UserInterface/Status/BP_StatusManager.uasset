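; BP_StatusManager exposes ratios for three status resources (HP, MP and Identity), filed under the game's status UI.
; Each getter divides the current value by its maximum, with no clamping or explicit zero check on the maximum.
; The file contains only these getters and no logic that sets or updates the values.
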(fn `GetHPRatio`
  (returns (Ratio :type "Float (double-precision)"))
  (return (/ (`self.CurrentHP`) (`self.MaxHP`))))

(fn `GetIdentityRatio`
  (returns (Ratio :type "Float (double-precision)"))
  (return (/ (`self.CurrentIdentity`) (`self.MaxIdentity`))))

(fn `GetMPRatio`
  (returns (Ratio :type "Float (double-precision)"))
  (return (/ (`self.CurrentMP`) (`self.MaxMP`))))